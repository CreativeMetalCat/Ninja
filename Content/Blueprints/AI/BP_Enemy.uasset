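; Enemy Blueprint that acts as the victim of paired attack animations, such as those used for kills.
; When attacked, it snaps to the attacker's victim transform, plays the victim montage looked up by attack name in DT_Attacks, and disables capsule collision.
; A "Death" montage notify switches the mesh to ragdoll physics and calls Die, which runs the parent logic and plays Death.
; The stealth-kill check defers to the parent.
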(event EventBeginPlay)

(event Collision|EventActorBeginOverlap
  (params (OtherActor :type Actor%20Object%20Reference)))

(event EventTick
  (params (DeltaSeconds :type Float%20%28single-precision%29)))

(event EventBeAttacked
  (params (Attacker :type Ninja%20Character%20Base%20Object%20Reference) (AttackName :type Name :default "None"))
  (bind _mesh (Variables|Character|GetMesh))
  (bind _returnvalue (Class|NinjaCharacterBase|GetVictimTransform Attacker))
  (Transformation|SetActorLocation (.Location (Math|Transform|BreakTransform _returnvalue)) false false)
  (Transformation|SetActorRotation (.Rotation (Math|Transform|BreakTransform _returnvalue)))
  (bind _returnvalue_2 (Utilities|GetDataTableRow "/Game/Blueprints/AttackSystem/DT_Attacks.DT_Attacks" AttackName)
    (:then
      (bind _notifyname (Animation|Montage|PlayMontage (Variables|Character|GetMesh) (.VictimAnim (Utilities|Struct|BreakS_Attack _returnvalue_2)))
        (:then
          (Collision|SetCollisionEnabled (Variables|Default|GetCapsuleComponent) "NoCollision"))
        (:OnNotifyBegin
          (if (Utilities|Name|Equal(Name) _notifyname "Death")
            (Collision|SetCollisionEnabled _mesh "QueryAndPhysics")
            (Physics|SetSimulatePhysics _mesh true)
            (Class|NinjaCharacterBase|Die)))))))

(event EventDie
  (|CallParentFunction)
  (Audio|Components|Audio|Play (Variables|Default|GetDeath) 0.0))

(fn ConstructionScript)

(fn CanbeStealthKilled
  (bind _returnvalue (|CallParentFunction))
  (return _returnvalue))