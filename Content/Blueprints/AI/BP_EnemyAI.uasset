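; BP_EnemyAI is an enemy AI controller that runs the enemy soldier behavior tree and selects a patrol point on begin play.
; Every tick it polls its AIPerception component, sending heard actors to UpdateHeardActors and seen actors to UpdateAI, neither of which is defined here.
; GetCorrectPerceptionComponent exposes that perception component.
; An unconnected loop over last sensed stimuli never runs.
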(event EventBeginPlay
  (AI|RunBehaviorTree "/Game/Blueprints/AI/BT_EnemySolder.BT_EnemySolder")
  (Class|EnemyAIBase|SelectNextPatrolPoint))

(event EventTick
  (params (DeltaSeconds :type Float%20%28single-precision%29))
  (bind _aiperception (Variables|Default|GetAIPerception))
  (Class|EnemyAIBase|UpdateHeardActors (Class|AIPerceptionComponent|GetPerceivedActors _aiperception "/Script/AIModule.AISense_Hearing"))
  (Class|EnemyAIBase|UpdateAI (Class|AIPerceptionComponent|GetPerceivedActors _aiperception "/Script/AIModule.AISense_Sight")))

(fn ConstructionScript)

(fn GetCorrectPerceptionComponent
  (return (Variables|Default|GetAIPerception)))