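; Interactable diesel generator that toggles on and off and emits "Distraction"-tagged AI noise while running.
; Interact flips Activated, which starts or stops the engine audio and a looping timer that calls MakeNoise at the actor's location.
; BeginPlay applies the initial Activated state through the same branch without toggling it.
; The construction script sizes SoundSphere to the noise Range.
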(event Custom|SpawnNoise
  (Class|Actor|MakeNoise 1.0 0 (Transformation|GetActorLocation) (Variables|Default|GetRange) "Distraction"))

(event EventBeginPlay
  (bind _diesel_engine_idle1_cue (Variables|Default|Getdiesel_engine_idle1_Cue))
  (if (stale EventInteract _output_get)
    (Audio|Components|Audio|Play _diesel_engine_idle1_cue 0.0)
    (bind _returnvalue (Utilities|Time|SetTimerbyEvent (delegate Custom|SpawnNoise) (Variables|Default|GetNoiseSpawnInterval) true))
    (Variables|Default|SetNoiseSpawnTimerHandle _returnvalue)
    (else
      (Audio|Components|Audio|Stop _diesel_engine_idle1_cue)
      (Utilities|Time|ClearandInvalidateTimerbyHandle (Variables|Default|GetNoiseSpawnTimerHandle)))))

(event Collision|EventActorBeginOverlap
  (params (OtherActor :type Actor%20Object%20Reference)))

(event EventTick
  (params (DeltaSeconds :type Float%20%28single-precision%29)))

(event EventInteract
  (params (interactor :type Actor%20Object%20Reference))
  (bind _diesel_engine_idle1_cue (Variables|Default|Getdiesel_engine_idle1_Cue))
  (bind _output_get (Variables|Default|SetActivated (not (Variables|Default|GetActivated))))
  (if _output_get
    (Audio|Components|Audio|Play _diesel_engine_idle1_cue 0.0)
    (bind _returnvalue (Utilities|Time|SetTimerbyEvent (delegate Custom|SpawnNoise) (Variables|Default|GetNoiseSpawnInterval) true))
    (Variables|Default|SetNoiseSpawnTimerHandle _returnvalue)
    (else
      (Audio|Components|Audio|Stop _diesel_engine_idle1_cue)
      (Utilities|Time|ClearandInvalidateTimerbyHandle (Variables|Default|GetNoiseSpawnTimerHandle)))))

(fn ConstructionScript
  (Components|Sphere|SetSphereRadius (Variables|Default|GetSoundSphere) (Variables|Default|GetRange) false))