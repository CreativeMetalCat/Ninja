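; BP_Character_B is a character Blueprint in the MedicalWorker01 folder, assembled from a main skeletal mesh and five accessory mesh components.
; On BeginPlay, it sets the main SkeletalMeshComponent as master pose for Acc01 through Acc05, so the accessories follow the body's pose.
; The construction script is empty, so this link is made only at runtime, and the graphs hold no other logic.
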(event EventBeginPlay
  (bind _skeletalmeshcomponent (Variables|SkeletalMeshActor|GetSkeletalMeshComponent))
  (Class|SkinnedMeshComponent|SetMasterPoseComponent (Variables|Default|GetAcc01) _skeletalmeshcomponent)
  (Class|SkinnedMeshComponent|SetMasterPoseComponent (Variables|Default|GetAcc02) _skeletalmeshcomponent)
  (Class|SkinnedMeshComponent|SetMasterPoseComponent (Variables|Default|GetAcc03) _skeletalmeshcomponent)
  (Class|SkinnedMeshComponent|SetMasterPoseComponent (Variables|Default|GetAcc04) _skeletalmeshcomponent)
  (Class|SkinnedMeshComponent|SetMasterPoseComponent (Variables|Default|GetAcc05) _skeletalmeshcomponent))

(fn ConstructionScript)